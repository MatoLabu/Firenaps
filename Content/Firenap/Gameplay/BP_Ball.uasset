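; BP_Ball is a short-lived glowing, colored ball that can burst like a firework.
; Construction gives its sphere a bright dynamic emissive material, picking a random color unless one is set.
; A timeline stretched to its Life scales it along a fade-out curve, then expires the actor.
; On EndPlay, if SpawnAtEnd is set, it has the GM spawn a random number of smaller, same-colored fireballs at its location.
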(event `self.ReceiveEndPlay`
  (params (EndPlayReason :type "EEndPlayReason Enum" :default "Destroyed"))
  (if (`self.SpawnAtEnd`)
    (for _ (range 1 (+ (`KismetMathLibrary.RandomIntegerInRange` 10 500) 1))
      (`/Game/Firenap/Gameplay/BP_GameMode.SpawnFireBalls` :`self` (`/Game/Firenap/BPFL_FunctionLibrary.GetGM`) :`Location` (`self.K2_GetActorLocation`) :`RandomRotator` true :`Lifespan` (`KismetMathLibrary.RandomFloatInRange` 2.9 3.1) :`Force` 100.0 :`SetColor` true :`Color` (`self.Color`) :`Scale` 0.5))))

(event `self.ReceiveBeginPlay`
  (set `self.InitialScale` (`self.GetActorScale3D`))
  (`TimelineComponent.SetTimelineLength` (`self.T_Life`) (`self.Life`))
  (`Timeline|T_Life` :!via `PlayFromStart`
    (:`Update`
      (`self.SetActorScale3D` (* (`self.InitialScale`) (`CurveFloat.GetFloatValue` (`self.CRV_FadeOut`) (`/Game/Firenap/BPFL_FunctionLibrary.GetTimelinePercentage` (`self.T_Life`))))))
    (:`Finished`
      (`self.SetLifeSpan` 0.01))))

(fn `UserConstructionScript`
  (bind _returnvalue (`PrimitiveComponent.CreateDynamicMaterialInstance` (`self.Sphere`) 0 "/Game/Firenap/M_SimpleEmissive_Inst.M_SimpleEmissive_Inst"))
  (if (not (`self.SetColor`))
    (set `self.Color` (`KismetMathLibrary.MakeColor` (`KismetMathLibrary.RandomFloatInRange` 0.0 1.0) (`KismetMathLibrary.RandomFloatInRange` 0.0 1.0) (`KismetMathLibrary.RandomFloatInRange` 0.0 1.0))))
  (`MaterialInstanceDynamic.SetVectorParameterValue` _returnvalue "Color" (`self.Color`))
  (`MaterialInstanceDynamic.SetScalarParameterValue` _returnvalue "Multiply" 1000.0))