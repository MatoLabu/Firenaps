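; BP_Canon is a cannon that launches bursts of fireballs on its own at random intervals, or when the left mouse button is pressed.
; Each burst randomly tilts the Cylinder before every shot, then has the GM spawn a fireball at the Arrow's transform with randomized force and lifespan.
; BeginPlay starts an endless loop that waits a random delay, fires a random-sized burst, then re-arms itself.
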(event `Key|LeftMouseButton`
  (params (Key :type "Key Structure"))
  (bind (_returnvalue_location _returnvalue_rotation) (`KismetMathLibrary.BreakTransform` (`SceneComponent.K2_GetComponentToWorld` (`self.Arrow`))))
  (:`Pressed`
    (for _ (range 1 (+ (`KismetMathLibrary.RandomIntegerInRange` 1 50) 1)) :!label _label
      (`SceneComponent.K2_SetRelativeRotation` (`self.Cylinder`) (`KismetMathLibrary.MakeRotator` (`KismetMathLibrary.RandomFloatInRange` -30.0 30.0)) false false)
      (`/Game/Firenap/Gameplay/BP_GameMode.SpawnFireBalls` :`self` (`/Game/Firenap/BPFL_FunctionLibrary.GetGM`) :`Location` _returnvalue_location :`Rotator` _returnvalue_rotation :`ChildrenProba` 1.0 :`Lifespan` (`KismetMathLibrary.RandomFloatInRange` 3.0 4.0) :`Force` (`KismetMathLibrary.RandomFloatInRange` 250.0 1000.0) :`Scale` 0.5))))

(event `self.ReceiveBeginPlay`
  (`KismetSystemLibrary.Delay` (`KismetMathLibrary.RandomFloatInRange` 0.1 10.0) :!label _label_2)
  (`|ExecutionSequence`
    (:`then_0`
      (goto _label))
    (:`then_1`
      (goto _label_2))))

(fn `UserConstructionScript`)