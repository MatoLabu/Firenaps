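; Game mode for Firenap that provides a shared SpawnFireBalls function for creating and launching BP_Ball actors.
; Each ball gets a given or random rotation, plus scale, color, lifespan and a weighted-random SpawnAtEnd flag, apparently for child spawning.
; Its sphere receives a randomized forward impulse with a fixed upward boost.
; The event graph and construction script hold no logic.
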(fn `SpawnFireBalls`
  (params (Location :type "Vector Structure") (RandomRotator :type Boolean) (Rotator :type "Rotator Structure") (ChildrenProba :type "Float (double-precision)") (Lifespan :type "Float (double-precision)") (Force :type "Float (double-precision)") (SetColor :type Boolean) (Color :type "LinearColor Structure") (Scale :type "Float (double-precision)"))
  (bind _returnvalue (`|SpawnActorFromClass` "/Game/Firenap/Gameplay/BP_Ball.BP_Ball_C" (`KismetMathLibrary.MakeTransform` Location (select `bool` RandomRotator :`false` Rotator :`true` (`KismetMathLibrary.RandomRotator` false)) (`KismetMathLibrary.MakeVector` Scale Scale Scale)) "Undefined" "OverrideRootScale" null (`KismetMathLibrary.RandomBoolWithWeight` ChildrenProba) SetColor Color Lifespan null))
  (`PrimitiveComponent.AddImpulse` (`/Game/Firenap/Gameplay/BP_Ball.Sphere` _returnvalue) (+ (* (`self.GetActorForwardVector` _returnvalue) (* Force (`KismetMathLibrary.RandomFloatInRange` 3.0 5.0))) (0.0 0.0 1500.0)) "None" false)
  (`self.SetLifeSpan` _returnvalue Lifespan))

(fn `UserConstructionScript`)